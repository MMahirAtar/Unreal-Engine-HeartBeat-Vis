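; BP_HearthConnection is an actor that feeds a heart-pulse rate from a local socket connection into the material on its Plane.
; Connecting on BeginPlay, it prints each message's two-character string, converts it to the target rate and resets a timer value T.
; Tick smooths the rate and eases T back toward one, writing both to the dynamic material instance created in the Construction Script.
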(event Custom|Connected
  (params (ConnectionId :type Integer))
  (Variables|Default|SetConnectionID ConnectionId))

(event Custom|Message%20recived
  (params (ConnectionId :type Integer) (Message :type Array%20of%20Bytes))
  (bind _returnvalue (Class|TcpSocketConnection|MessageReadString Message 2))
  (Development|PrintString _returnvalue)
  (Variables|Default|SetRate (Math|Conversions|ToFloat(Integer) _returnvalue))
  (Variables|Default|SetT 0.0))

(event Custom|CustomEvent
  (params (ConnectionId :type Integer)))

(event EventBeginPlay
  (Class|TcpSocketConnection|Connect "127.0.0.1" 1234 (delegate Custom|CustomEvent) (delegate Custom|Connected) (delegate Custom|Message%20recived)))

(event Collision|EventActorBeginOverlap
  (params (OtherActor :type Actor%20Object%20Reference)))

(event EventTick
  (params (DeltaSeconds :type Float%20%28single-precision%29))
  (bind _output_get (Variables|Default|SetİnterpedRate (Math|Interpolation|FInterpTo (Variables|Default|GetİnterpedRate) (Variables|Default|GetRate) DeltaSeconds 4.0)))
  (Rendering|Material|SetScalarParameterValue (Variables|Default|GetDMI) "rate" _output_get :!class /Script/Engine.MaterialInstanceDynamic)
  (bind _output_get_2 (Variables|Default|SetT (Math|Interpolation|FInterpTo (Variables|Default|GetT) 1.0 DeltaSeconds 4.0)))
  (Rendering|Material|SetScalarParameterValue (Variables|Default|GetDMI) "t" _output_get_2 :!class /Script/Engine.MaterialInstanceDynamic))

(fn ConstructionScript
  (bind _plane (Variables|Default|GetPlane))
  (bind _returnvalue (Rendering|Material|CreateDynamicMaterialInstance _plane 0 (Rendering|Material|GetMaterial _plane 0) "None" :!class /Script/Engine.PrimitiveComponent))
  (bind _output_get (Variables|Default|SetDMI _returnvalue))
  (Rendering|Material|SetMaterial (Variables|Default|GetPlane) 0 _output_get))